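; Test Blueprint for filling a spline outline with a triangular point grid, left unfinished with an empty construction script.
; Disconnected construction nodes would draw arrows along the spline and place instanced meshes at the grid points.
; MakePointGrid sizes loops from spline bounds, but its live path only sets a placeholder location.
; Its unwired section classifies points as inside, edge or outside by cross/dot tests and distance, snapping edge points onto the spline.
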(fn ConstructionScript)

(fn MakePointGrid
  (params (In_Spline :type Spline%20Component%20Object%20Reference))
  (bind _ref_triangle_size (LocalVariables|GetREF_Triangle_Size))
  (bind _returnvalue (Math|Float|Clamp(Float) _ref_triangle_size 2.0 3e+01))
  (LocalVariables|SetREF_Spline In_Spline)
  (LocalVariables|SetNum_X (Math|Float|Ceil (+ (/ (.x (.BoxExtent (Collision|GetComponentBounds (LocalVariables|GetREF_Spline)))) _returnvalue) 1.0)))
  (LocalVariables|SetNum_Y (Math|Float|Ceil (+ (/ (.y (.BoxExtent (Collision|GetComponentBounds (LocalVariables|GetREF_Spline)))) (* (/ _returnvalue 2.0) (Math|Trig|Tan(Degrees) (LocalVariables|Get60_Degree)))) 1.0)))
  (for _index (range (* (LocalVariables|GetNum_Y) -1) (LocalVariables|GetNum_Y))
    (LocalVariables|SetIndex_Y _index)
    (for _index_2 (range (* (LocalVariables|GetNum_X) -1) (LocalVariables|GetNum_X))
      (LocalVariables|SetIndex_Y _index_2)
      (LocalVariables|SetCurrent_Location (Math|Vector|MakeVector 0.0 0.0 (.z (.Origin (Collision|GetComponentBounds (LocalVariables|GetREF_Spline)))))))))