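; BP_Planar_Volumes is a volume Blueprint that creates a dynamic MAT_Planar material on BeginPlay, setting a default color and low opacity.
; That startup path never assigns the material to a mesh.
; Disconnected, never-run logic counts overlapping BP_Planar_Anchor actors, maps their first tags to colors, and blends blue toward the first color by anchor count over a limit.
; That unused logic also applies the opaque material to the Sphere.
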(event EventBeginPlay
  (bind _returnvalue (Rendering|Material|CreateDynamicMaterialInstance "/FF_Contents/Planar/Assets/Materials/MAT_Planar.MAT_Planar" "None" "None" :!class /Script/Engine.KismetMaterialLibrary))
  (Variables|References|SetREF_MI _returnvalue)
  (Rendering|Material|SetVectorParameterValue (Variables|References|GetREF_MI) "Color" (Variables|Default|GetDefault_Color) :!class /Script/Engine.MaterialInstanceDynamic)
  (Rendering|Material|SetScalarParameterValue (Variables|References|GetREF_MI) "Opacity" 0.25 :!class /Script/Engine.MaterialInstanceDynamic))

(fn ConstructionScript)