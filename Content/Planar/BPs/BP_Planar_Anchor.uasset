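; BP_Planar_Anchor is a planar anchor actor shown as a cone mesh with configurable color, opacity and type.
; Construction script and BeginPlay both create a dynamic instance of MAT_Planar, then run the color and type setup functions.
; FSetColor pushes Opacity and Color into that instance and applies it to the cone.
; FSetType replaces the actor's Tags with its Type, so the anchor is identifiable by tag.
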(event EventBeginPlay
  (bind _returnvalue (Rendering|Material|CreateDynamicMaterialInstance "/FF_Contents/Planar/Assets/Materials/MAT_Planar.MAT_Planar" "None" "None" :!class /Script/Engine.KismetMaterialLibrary))
  (Variables|Referances|SetREF_MI _returnvalue)
  (CallFunction|FSetColor)
  (CallFunction|FSetType))

(fn ConstructionScript
  (bind _returnvalue (Rendering|Material|CreateDynamicMaterialInstance "/FF_Contents/Planar/Assets/Materials/MAT_Planar.MAT_Planar" "None" "None" :!class /Script/Engine.KismetMaterialLibrary))
  (Variables|Referances|SetREF_MI _returnvalue)
  (CallFunction|FSetColor)
  (CallFunction|FSetType))

(fn FSetColor
  (Rendering|Material|SetScalarParameterValue (Variables|Referances|GetREF_MI) "Opacity" (Variables|Instances|GetOpacity) :!class /Script/Engine.MaterialInstanceDynamic)
  (Rendering|Material|SetVectorParameterValue (Variables|Referances|GetREF_MI) "Color" (Variables|Instances|GetColor) :!class /Script/Engine.MaterialInstanceDynamic)
  (Rendering|Material|SetMaterial (Variables|Default|GetSM_Planar_Cone) 0 (Variables|Referances|GetREF_MI))
  (return))

(fn FSetType
  (Variables|Default|SetTags (Utilities|Array|MakeArray (Variables|Instances|GetType)))
  (return))